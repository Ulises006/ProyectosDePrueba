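; ActorB is an Actor Blueprint that prints its own character-style stats to the screen when play begins.
; BeginPlay concatenates its variables for name, life, resistance, damage, critical damage, speed and rotation speed into one string, shown for ten seconds with empty separators between values.
; Overlap and Tick events are disabled placeholders, and the construction script is empty.
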(event EventBeginPlay
  (Development|PrintString (Utilities|String|Append (Variables|Default|Getnombre) " 
" (Utilities|String|ToString(Float) (Variables|Default|Getvida)) " 
" (Utilities|String|ToString(Float) (Variables|Default|Getresistencia)) " 
" (Utilities|String|ToString(Integer) (Variables|Default|Getdaño)) " 
" (Utilities|String|ToString(Float) (Variables|Default|Getdaño%20critico)) " 
" (Utilities|String|ToString(Vector) (Variables|Default|Getvelocidad)) " 
" (Utilities|String|ToString(Rotator) (Variables|Default|Getvelrotacion))) true true "(R=0.000000,G=0.660000,B=1.000000,A=1.000000)" 1e+01))

(event Collision|EventActorBeginOverlap
  (params (OtherActor :type Actor%20Object%20Reference)))

(event EventTick
  (params (DeltaSeconds :type Float%20%28single-precision%29)))

(fn ConstructionScript)